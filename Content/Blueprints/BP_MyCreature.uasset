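; BP_MyCreature is a 2D flipbook creature driven by an animation state and a facing direction.
; BeginPlay loads its data, including flipbooks, from a data table row keyed by CreatureName.
; Each tick it sets the flipbook matching AniStatus, then runs horizontally along X by Direction or jumps.
; UpdateDirection is an empty stub, and nothing in this Blueprint changes AniStatus or Direction.
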(event `self.ReceiveBeginPlay`
  ;[1 1 1] Set Creature Data
  (bind _returnvalue (`|GetDataTableRow` "/Game/Blueprints/Data/CreatureDataTable.CreatureDataTable" (`self.CreatureName`))
    (:`then`
      (set `self.CreatureData` _returnvalue))))

(event `self.ReceiveTick`
  (params (DeltaSeconds :type "Float (single-precision)"))
  (`self.UpdateDirection`)
  (`self.UpdateAnimation`)
  (`self.UpdateMove`))

(fn `UpdateAnimation`
  (bind (_creaturedata_maxhp _creaturedata_damage _creaturedata_flipbooks) (break `/Game/Blueprints/Data/CreatureData` (`self.CreatureData`)))
  (bind (_idle _run _attack _jump) (break `/Game/Blueprints/Data/FlipbookData` _creaturedata_flipbooks))
  (`PaperFlipbookComponent.SetFlipbook` (`self.Sprite`) (select `/Game/Blueprints/EAniStatus` (`self.AniStatus`) :`NewEnumerator0` _idle :`NewEnumerator1` _run :`NewEnumerator2` _attack :`NewEnumerator4` _jump)))

(fn `UpdateDirection`)

(fn `UpdateMove`
  (switch `/Game/Blueprints/EAniStatus` (`self.AniStatus`)
    (:`NewEnumerator1`
      (switch `/Game/Blueprints/Direction` (`self.Direction`)
        (:`NewEnumerator0`
          (`self.AddMovementInput` (-1.0 0.0 0.0)))
        (:`NewEnumerator1`
          (`self.AddMovementInput` (1.0 0.0 0.0)))))
    (:`NewEnumerator4`
      (`self.Jump`))))

(fn `UserConstructionScript`)