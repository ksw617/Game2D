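; BP_MyPlayer is the player Blueprint that switches a 2D sprite between idle and run flipbooks from left/right input.
; The MoveLeftRight axis event stores the input and sets an Idle or Run animation status, which then selects the flipbook.
; While running, it mirrors the sprite by scaling X with the signed axis value, so partial input also narrows it.
; The graph applies no movement itself.
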(event `InputAxis|MoveLeftRight`
  (params (AxisValue :type "Float (single-precision)"))
  (bind _sprite (`self.Sprite`))
  ;[1 1 1] Set Value
  (bind _output_get (set `self.MoveAxis` AxisValue))
  (set `self.Run` (> (`KismetMathLibrary.Abs` _output_get) 0.0))
  (`|ExecutionSequence`
    (:`then_0`
      ;[1 1 1] Set Animation Status
      (if (`self.Run`)
        (set `self.AniStatus` "NewEnumerator1")
        (`SceneComponent.SetRelativeScale3D` (`self.Sprite`) (`KismetMathLibrary.MakeVector` (* (`self.MoveAxis`) 2.0) 2.0 2.0))
        (else
          (set `self.AniStatus` "NewEnumerator0"))))
    (:`then_1`
      ;[1 1 1] Set Flipbook Animation
      (switch `/Game/Blueprints/EAniStatus` (`self.AniStatus`)
        (:`NewEnumerator0`
          (`PaperFlipbookComponent.SetFlipbook` _sprite "/Game/PixelHeroVol1/idle.idle"))
        (:`NewEnumerator1`
          (`PaperFlipbookComponent.SetFlipbook` _sprite "/Game/PixelHeroVol1/run.run"))))))

(fn `UserConstructionScript`)