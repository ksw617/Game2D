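; BP_MyEnemy is an enemy that chases and attacks the player along one horizontal axis.
; After the parent Tick, it switches on AniStatus: Idle finds BP_MyPlayer with GetActorOfClass and changes to Run once the target is valid.
; Run fires AttackEvent within a short range, otherwise sets MoveLeftRight to the X of the normalized direction to the target.
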(event `self.ReceiveTick`
  (params (DeltaSeconds :type "Float (single-precision)"))
  (bind _target (`self.Target`))
  (bind _returnvalue_x (`KismetMathLibrary.BreakVector` (`KismetMathLibrary.Normal` (`self.Direction`))))
  (`parent.ReceiveTick` DeltaSeconds)
  (switch `/Game/Blueprints/EAniStatus` (`self.AniStatus`)
    (:`NewEnumerator0`
      (bind _returnvalue (`GameplayStatics.GetActorOfClass` "/Game/Blueprints/BP_MyPlayer.BP_MyPlayer_C"))
      (bind _output_get (set `self.Target` _returnvalue))
      (`/Engine/EditorBlueprintResources/StandardMacros.IsValid` _output_get
        (:`Is Valid`
          (set `self.AniStatus` "NewEnumerator1"))))
    (:`NewEnumerator1`
      (`/Engine/EditorBlueprintResources/StandardMacros.IsValid` _target
        (:`Is Valid`
          (bind _output_get_2 (set `self.Direction` (- (`self.K2_GetActorLocation` _target) (`self.K2_GetActorLocation` self))))
          (if (< (`KismetMathLibrary.VSize` _output_get_2) 200.0)
            (`self.AttackEvent`)
            (else
              (set `self.MoveLeftRight` _returnvalue_x))))))))

(fn `UserConstructionScript`
  (`parent.UserConstructionScript`))